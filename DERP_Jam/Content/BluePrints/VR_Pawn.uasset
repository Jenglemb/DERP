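; VR pawn that lets the player interact with world objects using either hand, with floor-level tracking.
; Each hand's interact input searches that hand's grab sphere for the nearest overlapping actor implementing Interract_Interface and sends it InterractMessage.
; It then prints a debug message and clears the launch-button flag if set, otherwise printing the incoming prime value.
; BeginPlay also resets that flag and clears the location prime values.
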(event EventBeginPlay
  (Class|HeadMountedDisplayFunctionLibrary|SetTrackingOrigin "Floor")
  (Variables|Default|SetbLaunchButtonActive false)
  (Utilities|Array|Clear (Variables|Default|GetLocationPrimeValues)))

(event Input|ActionEvents|InputActionInterract_L
  (params (Key :type Key%20Structure :default "AnyKey"))
  (:Pressed
    (Grabbing|InterractL)))

(event Input|ActionEvents|InputActionInterract_R
  (params (Key :type Key%20Structure :default "AnyKey"))
  (:Pressed
    (Grabbing|InterractR)))

(fn ConstructionScript)

(fn InterractR
  (Variables|Default|SetR_WantsToGrab true)
  (bind _nearestmesh (Grabbing|GetActorNearHandR))
  (Utilities|IsValid _nearestmesh
    (:Is%20Valid
      (Variables|Default|SetCurrentActor 0)
      (Class|InterractInterface|Interract(Message) _nearestmesh)
      (if (Variables|Default|GetbLaunchButtonActive)
        (Development|PrintString "DONKEY: LaunchButtonCalled")
        (Variables|Default|SetbLaunchButtonActive false)
        (else
          (Development|PrintString (Utilities|String|ToString(Integer) (Variables|Default|GetPrimeValueIn))))))))

(fn InterractL
  (Variables|Default|SetL_WantsToGrab true)
  (bind _nearestmesh (Grabbing|GetActorNearHandL))
  (Utilities|IsValid _nearestmesh
    (:Is%20Valid
      (Class|InterractInterface|Interract(Message) _nearestmesh)
      (if (Variables|Default|GetbLaunchButtonActive)
        (Development|PrintString "DONKEY: LaunchButtonCalled")
        (Variables|Default|SetbLaunchButtonActive false)
        (else
          (Development|PrintString (Utilities|String|ToString(Integer) (Variables|Default|GetPrimeValueIn))))))))

(fn GetActorNearHandR
  (bind _r_grabsphere (Variables|Default|GetR_GrabSphere))
  (for _array_element (Collision|GetOverlappingActors _r_grabsphere "/Script/Engine.Actor" :!class /Script/Engine.PrimitiveComponent)
    (if (Utilities|DoesObjectImplementInterface _array_element "/Game/BluePrints/Interract_Interface.Interract_Interface_C")
      (if (< (Math|Vector|VectorLength (- (Transformation|GetActorLocation _array_element) (Transformation|GetWorldLocation _r_grabsphere))) (LocalVariables|GetNearestOverlap))
        (LocalVariables|SetNearestOverlappingActor _array_element)
        (LocalVariables|SetNearestOverlap (Math|Vector|VectorLength (- (Transformation|GetActorLocation _array_element) (Transformation|GetWorldLocation _r_grabsphere)))))))
  (return (LocalVariables|GetNearestOverlappingActor)))

(fn GetActorNearHandL
  (bind _l_grabsphere (Variables|Default|GetL_GrabSphere))
  (for _array_element (Collision|GetOverlappingActors _l_grabsphere "/Script/Engine.Actor" :!class /Script/Engine.PrimitiveComponent)
    (if (Utilities|DoesObjectImplementInterface _array_element "/Game/BluePrints/Interract_Interface.Interract_Interface_C")
      (if (< (Math|Vector|VectorLength (- (Transformation|GetWorldLocation _l_grabsphere) (Transformation|GetActorLocation _array_element))) (LocalVariables|GetNearestOverlap))
        (LocalVariables|SetNearestOverlappingActor _array_element)
        (LocalVariables|SetNearestOverlap (Math|Vector|VectorLength (- (Transformation|GetWorldLocation _l_grabsphere) (Transformation|GetActorLocation _array_element)))))))
  (return (LocalVariables|GetNearestOverlappingActor)))